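; BP_Player is the player Blueprint, providing a camera transition to a cinematic view and a honk notification.
; TransitionToCineCam plays a timeline, commented as five seconds, that lerps the camera from its current world transform toward a CineCameraActor's camera, setting InCineCam to block retriggering.
; Honk maps its pitch type, Low through High, to an integer and broadcasts it through the OnHonk dispatcher.
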(event Custom|Honk
  (params (honktype :type E_HonkType%20Enum :default "NewEnumerator0"))
  (Default|CallOnHonk (Utilities|Select :Index honktype :NewEnumerator0 (Class|KismetSystemLibrary|MakeLiteralInteger 1) :NewEnumerator1 2 :NewEnumerator2 3 :NewEnumerator3 4)))

(event Custom|TransitionToCineCam
  (bind _camera (Variables|Default|GetCamera))
  ;[1 1 1] Trasforms the starting camera to be the CineCam Actor's transformation over 5 second
  (if (not (Variables|Default|GetInCineCam))
    (bind _returnvalue (Actor|GetActorOfClass "/Script/CinematicCamera.CineCameraActor"))
    (bind _output (Timeline|Transition PlayFromStart)
      (:Update
        (Transformation|SetWorldTransform _camera (Math|Transform|Lerp(Transform) (Transformation|GetWorldTransform _camera) (Transformation|GetWorldTransform (Variables|/Script/Engine.CameraActor|GetCameraComponent _returnvalue)) _output) false false)
        (Variables|Default|SetInCineCam true)))))

(fn ConstructionScript
  (|CallParentFunction))