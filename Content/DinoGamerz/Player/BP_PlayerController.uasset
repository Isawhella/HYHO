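; Player controller for a goose honking game that handles the start flow, honk input, HUD and pausing.
; StartGame swaps the start widget for the HUD after a cine cam transition, then calls GameStart on BP_GameMode.
; Four honk inputs each set the ABP_GooseAnimations enum and call Honk on BP_Player, with ReturnToIdle resetting the animation.
; HUD and pause widgets are created once from game mode classes.
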(event Custom|AddHud
  ;[1 1 1] add HUD
  (Utilities|IsValid (Variables|Default|GetHudRef)
    (:Is%20Valid
      _)
    (:Is%20Not%20Valid
      (bind _asbp_game_mode (Utilities|Casting|CastToBP_GameMode (Game|GetGameMode))
        (:then
          _)
        (:CastFailed
          _))
      (bind _returnvalue (UserInterface|CreateWidget (Variables|/Game/DinoGamerz/Player/BP_GameMode.BP_GameMode_C|GetGameHud _asbp_game_mode) self))
      (bind _output_get (Variables|Default|SetHudRef _returnvalue))))
  (UserInterface|Viewport|AddtoViewport _output_get 0))

(event Custom|ReturnToIdle
  (bind _asabp_goose_animations (Utilities|Casting|CastToABP_GooseAnimations (Components|SkeletalMesh|GetAnimInstance (Variables|/Script/Engine.Character|GetMesh (Variables|Default|GetPlayerRef)))))
  (Variables|/Game/DinoGamerz/Player/anim/ABP_GooseAnimations.ABP_GooseAnimations_C|SetGooseAnimationEnum _asabp_goose_animations "NewEnumerator4"))

(event EventBeginPlay
  (bind _returnvalue (UserInterface|CreateWidget "/Game/DinoGamerz/Widgets/W_StartGame.W_StartGame_C" self))
  (bind _output_get (Variables|Default|SetStartGameHudRef _returnvalue))
  (UserInterface|Viewport|AddtoViewport _output_get 0)
  (bind _returnvalue_2 (Actor|GetActorOfClass "/Game/DinoGamerz/Player/BP_Player.BP_Player_C"))
  (Variables|Default|SetPlayerRef _returnvalue_2))

(event Input|ActionEvents|InputActionHonk1
  (params (Key :type Key%20Structure))
  (:Pressed
    (bind _asabp_goose_animations (Utilities|Casting|CastToABP_GooseAnimations (Components|SkeletalMesh|GetAnimInstance (Variables|/Script/Engine.Character|GetMesh (Variables|Default|GetPlayerRef)))))
    (Variables|/Game/DinoGamerz/Player/anim/ABP_GooseAnimations.ABP_GooseAnimations_C|SetGooseAnimationEnum _asabp_goose_animations "NewEnumerator0")))

(event Input|ActionEvents|InputActionHonk2
  (params (Key :type Key%20Structure))
  (:Pressed
    (bind _asabp_goose_animations (Utilities|Casting|CastToABP_GooseAnimations (Components|SkeletalMesh|GetAnimInstance (Variables|/Script/Engine.Character|GetMesh (Variables|Default|GetPlayerRef)))))
    (Variables|/Game/DinoGamerz/Player/anim/ABP_GooseAnimations.ABP_GooseAnimations_C|SetGooseAnimationEnum _asabp_goose_animations "NewEnumerator1")))

(event Input|ActionEvents|InputActionHonk3
  (params (Key :type Key%20Structure))
  (:Pressed
    (bind _asabp_goose_animations (Utilities|Casting|CastToABP_GooseAnimations (Components|SkeletalMesh|GetAnimInstance (Variables|/Script/Engine.Character|GetMesh (Variables|Default|GetPlayerRef)))))
    (Variables|/Game/DinoGamerz/Player/anim/ABP_GooseAnimations.ABP_GooseAnimations_C|SetGooseAnimationEnum _asabp_goose_animations "NewEnumerator2")))

(event Input|ActionEvents|InputActionHonk4
  (params (Key :type Key%20Structure))
  (:Pressed
    (bind _asabp_goose_animations (Utilities|Casting|CastToABP_GooseAnimations (Components|SkeletalMesh|GetAnimInstance (Variables|/Script/Engine.Character|GetMesh (Variables|Default|GetPlayerRef)))))
    (Variables|/Game/DinoGamerz/Player/anim/ABP_GooseAnimations.ABP_GooseAnimations_C|SetGooseAnimationEnum _asabp_goose_animations "NewEnumerator3")))

(event Input|ActionEvents|InputActionPause
  (params (Key :type Key%20Structure))
  ;[1 1 1] pause
  (:Pressed
    (Utilities|IsValid (Variables|Default|GetPauseScreenRef)
      (:Is%20Valid
        _)
      (:Is%20Not%20Valid
        (bind _asbp_game_mode (Utilities|Casting|CastToBP_GameMode (Game|GetGameMode))
          (:then
            _)
          (:CastFailed
            _))
        (bind _returnvalue (UserInterface|CreateWidget (Variables|/Game/DinoGamerz/Player/BP_GameMode.BP_GameMode_C|GetPauseScreen _asbp_game_mode) self))
        (bind _output_get (Variables|Default|SetPauseScreenRef _returnvalue))))
    (UserInterface|Viewport|AddtoViewport _output_get 5)
    (Game|SetGamePaused true)))

(event Input|ActionEvents|InputActionHonk1
  (params (Key :type Key%20Structure))
  (:Pressed
    (CallFunction|PlayerHonk "NewEnumerator0")))

(event Input|ActionEvents|InputActionHonk2
  (params (Key :type Key%20Structure))
  (:Pressed
    (CallFunction|PlayerHonk "NewEnumerator1")))

(event Input|ActionEvents|InputActionHonk3
  (params (Key :type Key%20Structure))
  (:Pressed
    (CallFunction|PlayerHonk "NewEnumerator2")))

(event Input|ActionEvents|InputActionHonk4
  (params (Key :type Key%20Structure))
  (:Pressed
    (CallFunction|PlayerHonk "NewEnumerator3")))

(event Input|ActionEvents|InputActionStartGame
  (params (Key :type Key%20Structure))
  (:Pressed
    (if (not (Variables|Default|GetGameStarted))
      (Widget|RemovefromParent (Variables|Default|GetStartGameHudRef))
      (Default|TransitiontoCineCam (Variables|Default|GetPlayerRef))
      (Utilities|FlowControl|Delay 1.0)
      (CallFunction|AddHud)
      (Variables|Default|SetGameStarted true)
      (Utilities|FlowControl|Delay 0.5)
      (bind _asbp_game_mode (Utilities|Casting|CastToBP_GameMode (Game|GetGameMode)))
      (Default|GameStart _asbp_game_mode))))

(fn ConstructionScript
  (|CallParentFunction))

(fn PlayerHonk
  (params (honkType :type E_HonkType%20Enum :default "NewEnumerator0"))
  (bind _asbp_player (Utilities|Casting|CastToBP_Player (Pawn|GetControlledPawn)))
  (Default|Honk _asbp_player honkType))