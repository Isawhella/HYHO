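; BP_OtherGoose is a goose with four distinct honks, exposed as events for other code to trigger.
; Each honk event casts the skeletal mesh's anim instance to ABP_GooseAnimations, sets its animation enum and plays the matching GoodHonk sound in 2D.
; ReturnToIdle sets the same enum to its idle value without sound, leaving pose selection to the Animation Blueprint.
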(event Custom|ReturnToIdle
  (bind _asabp_goose_animations (Utilities|Casting|CastToABP_GooseAnimations (Components|SkeletalMesh|GetAnimInstance (Variables|Default|GetSkeletalMesh))))
  (Variables|/Game/DinoGamerz/Player/anim/ABP_GooseAnimations.ABP_GooseAnimations_C|SetGooseAnimationEnum _asabp_goose_animations "NewEnumerator4"))

(event Custom|Honk4
  (bind _asabp_goose_animations (Utilities|Casting|CastToABP_GooseAnimations (Components|SkeletalMesh|GetAnimInstance (Variables|Default|GetSkeletalMesh))))
  (Variables|/Game/DinoGamerz/Player/anim/ABP_GooseAnimations.ABP_GooseAnimations_C|SetGooseAnimationEnum _asabp_goose_animations "NewEnumerator3")
  (Audio|PlaySound2D "/Game/DinoGamerz/Audio/Honks/GoodHonks/GoodHonk4.GoodHonk4" 1.0 1.0 0.0 0 0))

(event Custom|Honk1
  (bind _asabp_goose_animations (Utilities|Casting|CastToABP_GooseAnimations (Components|SkeletalMesh|GetAnimInstance (Variables|Default|GetSkeletalMesh))))
  (Variables|/Game/DinoGamerz/Player/anim/ABP_GooseAnimations.ABP_GooseAnimations_C|SetGooseAnimationEnum _asabp_goose_animations "NewEnumerator0")
  (Audio|PlaySound2D "/Game/DinoGamerz/Audio/Honks/GoodHonks/GoodHonk1.GoodHonk1" 1.0 1.0 0.0 0 0))

(event Custom|Honk2
  (bind _asabp_goose_animations (Utilities|Casting|CastToABP_GooseAnimations (Components|SkeletalMesh|GetAnimInstance (Variables|Default|GetSkeletalMesh))))
  (Variables|/Game/DinoGamerz/Player/anim/ABP_GooseAnimations.ABP_GooseAnimations_C|SetGooseAnimationEnum _asabp_goose_animations "NewEnumerator1")
  (Audio|PlaySound2D "/Game/DinoGamerz/Audio/Honks/GoodHonks/GoodHonk2.GoodHonk2" 1.0 1.0 0.0 0 0))

(event Custom|Honk3
  (bind _asabp_goose_animations (Utilities|Casting|CastToABP_GooseAnimations (Components|SkeletalMesh|GetAnimInstance (Variables|Default|GetSkeletalMesh))))
  (Variables|/Game/DinoGamerz/Player/anim/ABP_GooseAnimations.ABP_GooseAnimations_C|SetGooseAnimationEnum _asabp_goose_animations "NewEnumerator2")
  (Audio|PlaySound2D "/Game/DinoGamerz/Audio/Honks/GoodHonks/GoodHonk3.GoodHonk3" 1.0 1.0 0.0 0 0))

(fn ConstructionScript)