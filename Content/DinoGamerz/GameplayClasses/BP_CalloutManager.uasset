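; BP_CalloutManager runs the call-and-response rhythm turns between the other goose and the player.
; SoundOffNotes recurses with tempo-scaled delays, adding each note to the HUD and triggering that goose's honks.
; PlayerResponse binds to player honks and steps through sixteenths, opening retriggerable-delay hit windows.
; Score reports hits and misses to the GameMode, off-window honks cost health, and dispatchers signal marks and turn completion.
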(event Custom|Sound%20Off%20Song
  (params (SongSeg :type S%20Song%20Seg%20Structure))
  (bind _returnvalue (Actor|GetActorOfClass "/Game/DinoGamerz/Player/BP_OtherGoose.BP_OtherGoose_C"))
  (Variables|Default|SetOtherGooseRef _returnvalue)
  (bind _output_get (Variables|Default|SetCurrentSongSeg SongSeg))
  (Utilities|FlowControl|DoOnce false
    (:Completed
      (bind (_valid _hudref) (CallFunction|IsValidSetup))
      (if (and _valid (> (Utilities|Array|Length (.Notes (Utilities|Struct|BreakS_Measure (.Rhythm (Utilities|Struct|BreakS_SongSeg _output_get))))) 0))
        (bind _asw_gameplay_hud (Utilities|Casting|CastToW_GameplayHud _hudref))
        (bind _asbp_game_mode (Utilities|Casting|CastToBP_GameMode (Game|GetGameMode)))
        (CallFunction|SoundOffNotes (.Notes (Utilities|Struct|BreakS_Measure (.Rhythm (Utilities|Struct|BreakS_SongSeg _output_get)))) (.Inputs (Utilities|Struct|BreakS_SongSeg _output_get)) (Class|KismetSystemLibrary|MakeLiteralInteger) (/ 6e+01 (Math|Conversions|ToFloat(Integer) (Variables|/Game/DinoGamerz/Player/BP_GameMode.BP_GameMode_C|GetTempo _asbp_game_mode))))))))

(event Custom|Sound%20off%20Notes
  (params (Notes :type Array%20of%20Integers) (Inputs :type Array%20of%20Integers) (note# :type Integer%20%28by%20ref%29) (BPS :type Float%20%28double-precision%29))
  (bind _output (Utilities|Array|Get(acopy) Notes note#))
  (bind _output_2 (Utilities|Array|Get(acopy) Inputs note#))
  (bind _othergooseref (Variables|Default|GetOtherGooseRef))
  ;[1 1 1] Recursive function; gives note to gameplay hud, pauses, and repeats on the next note (currently not working)
  (if (< note# (Utilities|Array|Length Notes))
    (Utilities|FlowControl|Sequence
      (:then_0
        (Default|AddNotetoMeasure (stale Custom|Sound%20Off%20Song _asw_gameplay_hud) _output _output_2)
        ;[1 1 1] honk the provided note (0 is rest; 1-4 are notes)
        (switch int _output_2
          (:1
            (CallFunction|PlayHonk "NewEnumerator0")
            (Default|Honk1 _othergooseref))
          (:2
            (CallFunction|PlayHonk "NewEnumerator1")
            (Default|Honk2 _othergooseref))
          (:3
            (CallFunction|PlayHonk "NewEnumerator2")
            (Default|Honk3 _othergooseref))
          (:4
            (CallFunction|PlayHonk "NewEnumerator3")
            (Default|Honk4 _othergooseref))))
      (:then_1
        ;[1 1 1] recurse with delay
        (Utilities|FlowControl|Delay (* (Math|Conversions|ToFloat(Integer) _output) BPS 0.25))
        (CallFunction|SoundOffNotes Notes Inputs (+ note# 1) BPS)))
    (else
      (Default|CallNoteReadFinished)
      (Utilities|FlowControl|DoOnce false) ; enters at Reset
    )))

(event Custom|PlayerResponse
  (params (length%2816ths%29 :type Integer) (BPS :type Float%20%28double-precision%29) (SongSeg :type S%20Song%20Seg%20Structure))
  ;[1 1 1] setup
  (if (not (Variables|Listening|GetPlayerInProgress))
    (Variables|Listening|SetPlayerInProgress true)
    (bind _asbp_player (Utilities|Casting|CastToBP_Player (Game|GetPlayerCharacter 0)))
    (EventDispatchers|BindEventtoOnHonk _asbp_player (delegate Custom|CustomEvent_0))
    ;[1 1 1] initial delay
    (Utilities|FlowControl|Delay (- (* (- length%2816ths%29 2) BPS 0.25) (/ (Variables|Default|Gethit%20window) 2.0)))
    (Variables|Listening|SetActiveListening false)
    (Variables|Listening|SetCurrentSongSeg_0 SongSeg)
    (Variables|Default|SetNextVal 0)
    (Variables|Listening|SetCurrentNote 0)
    (bind _index (Utilities|ForLoopwithDelay 0 length%2816ths%29 (/ BPS 4.0))
      (:LoopBody
        (if (> _index (Variables|Default|GetNextVal))
          (Variables|Default|SetintNoteIndex (Variables|Default|GetNextVal))
          (Variables|Default|SetNextVal (+ (Variables|Default|GetNextVal) (Utilities|Array|Get(acopy) (.Notes (Utilities|Struct|BreakS_Measure (.Rhythm (Utilities|Struct|BreakS_SongSeg (Variables|Listening|GetCurrentSongSeg_0))))) (Variables|Listening|GetCurrentNote))))
          (Variables|Listening|SetDesiredInput (Utilities|Array|Get(acopy) (.Inputs (Utilities|Struct|BreakS_SongSeg (Variables|Listening|GetCurrentSongSeg_0))) (Variables|Listening|GetCurrentNote)))
          (Math|Integer|IncrementInt (Variables|Listening|GetCurrentNote)
            (:%20%20
              (CallFunction|NoteWindow (Variables|Default|Gethit%20window))))))
      (:Completed
        (Variables|Listening|SetPlayerInProgress false)
        (bind _asbp_player_2 (Utilities|Casting|CastToBP_Player (Game|GetPlayerCharacter 0)))
        (EventDispatchers|UnbindEventfromOnHonk _asbp_player_2 (delegate Custom|CustomEvent_0))
        (CallFunction|EndPlayerTurn)))))

(event Custom|NoteWindow
  (params (Length :type Float%20%28double-precision%29))
  ;[1 1 1] open window for note
  (Utilities|FlowControl|Sequence
    (:then_0
      ;[1 1 1] Listen to honk
      (Utilities|FlowControl|DoOnce false) ; enters at Reset
    )
    (:then_1
      (if (Variables|Listening|GetActiveListening)
        (CallFunction|Score (Variables|Listening|GetnoteHitState))
        (else
          (Variables|Listening|SetActiveListening true)))
      (Variables|Listening|SetnoteHitState 0)
      (Utilities|FlowControl|RetriggerableDelay Length)
      (Variables|Listening|SetActiveListening false)
      (CallFunction|Score (Variables|Listening|GetnoteHitState)))))

(event Custom|Score
  (params (Hitstate :type Integer))
  ;[1 1 1] cast back to gamemode to score
  (bind _asbp_game_mode (Utilities|Casting|CastToBP_GameMode (Game|GetGameMode)))
  (switch int Hitstate
    (:Default
      (Variables|Listening|SetnoteHitState 0 :!label _label))
    (:0
      (Default|MissNote _asbp_game_mode :!label _label_2)
      (Default|CallMarkMiss (+ (Variables|Default|GetintNoteIndex) 2))
      (goto _label))
    (:1
      (Audio|SpawnSound2D "/Game/DinoGamerz/Audio/Honks/BadHonks/BadHonk3.BadHonk3" 1.0 1.0 0.0 0)
      (goto _label_2))
    (:2
      (Default|HitNote _asbp_game_mode)
      (Default|CallMarkHit (+ (Variables|Default|GetintNoteIndex) 2))
      (Utilities|FlowControl|Sequence
        (:then_0
          (switch int (Variables|Listening|GetDesiredInput)
            (:1
              (Audio|SpawnSound2D "/Game/DinoGamerz/Audio/Honks/GoodHonks/GoodHonk1.GoodHonk1" 1.0 1.0 0.0 0))
            (:2
              (Audio|SpawnSound2D "/Game/DinoGamerz/Audio/Honks/GoodHonks/GoodHonk2.GoodHonk2" 1.0 1.0 0.0 0))
            (:3
              (Audio|SpawnSound2D "/Game/DinoGamerz/Audio/Honks/GoodHonks/GoodHonk3.GoodHonk3" 1.0 1.0 0.0 0))
            (:4
              (Audio|SpawnSound2D "/Game/DinoGamerz/Audio/Honks/GoodHonks/GoodHonk4.GoodHonk4" 1.0 1.0 0.0 0))))
        (:then_1
          (goto _label))))))

(event Custom|CustomEvent_0
  (params (int :type Integer))
  ;[1 1 1] Listen to honk
  (if (Variables|Listening|GetActiveListening)
    (Utilities|FlowControl|DoOnce false
      (:Completed
        (Variables|Listening|SetnoteHitState (Math|Integer|SelectInt 2 1 (== (Variables|Listening|GetDesiredInput) int)))))
    (else
      (bind _asbp_game_mode (Utilities|Casting|CastToBP_GameMode (Game|GetGameMode)))
      (Variables|/Game/DinoGamerz/Player/BP_GameMode.BP_GameMode_C|SetHealth _asbp_game_mode (- (Variables|/Game/DinoGamerz/Player/BP_GameMode.BP_GameMode_C|GetHealth _asbp_game_mode) 2))
      (Audio|PlaySound2D "/Game/DinoGamerz/Audio/Honks/BadHonks/BadHonk2.BadHonk2" 1.0 1.0 0.0 0 0))))

(event Custom|End%20player%20turn
  (bind _asbp_player_controller (Utilities|Casting|CastToBP_PlayerController (Game|GetPlayerController 0)))
  (bind _asw_gameplay_hud (Utilities|Casting|CastToW_GameplayHud (Variables|/Game/DinoGamerz/Player/BP_PlayerController.BP_PlayerController_C|GetHudRef _asbp_player_controller)))
  (Default|ClearMeasure _asw_gameplay_hud)
  (Default|CallPlayerTurnFinished))

(fn ConstructionScript)

(fn IsValidSetup
  (bind _asbp_player_controller (Utilities|Casting|CastToBP_PlayerController (Game|GetPlayerController 0))
    (:then
      (Utilities|IsValid (Variables|/Game/DinoGamerz/Player/BP_PlayerController.BP_PlayerController_C|GetHudRef _asbp_player_controller)
        (:Is%20Valid
          (return true (Variables|/Game/DinoGamerz/Player/BP_PlayerController.BP_PlayerController_C|GetHudRef _asbp_player_controller)))
        (:Is%20Not%20Valid
          _)))
    (:CastFailed
      _))
  (return false 0))

(fn PlayHonk
  (params (HonkType :type E_HonkType%20Enum :default "NewEnumerator0"))
  (switch Utilities|FlowControl|Switch|SwitchonE_HonkType HonkType))